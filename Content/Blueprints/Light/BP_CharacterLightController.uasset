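; Character lighting controller Blueprint with a three-spotlight rig: front, back left and back right.
; The Construction Script copies the configured light colors and stage EV into current-state variables, then colors each spotlight from its own array entry.
; It sets intensity from the first entry of separate front and back arrays, with both back lights sharing one value.
; The event graph and the CharacterSpecularScale RepNotify are empty, so no runtime logic runs here.
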(fn `OnRep_CharacterSpecularScale`)

(fn `UserConstructionScript`
  (set `self.LightColorCurrent` (`self.LightColor`))
  (set `self.StageEV_current` (`self.StageEV`))
  (`LightComponent.SetLightColor` (`self.SpotLight_Front`) (`|GetArrayItem` (`self.LightColor`)) true)
  (`LightComponent.SetLightColor` (`self.SpotLight_BackLeft`) (`|GetArrayItem` (`self.LightColor`) 1) true)
  (`LightComponent.SetLightColor` (`self.SpotLight_BackRight`) (`|GetArrayItem` (`self.LightColor`) 2) true)
  (`LightComponent.SetIntensity` (`self.SpotLight_Front`) (`|GetArrayItem` (`self.LightIntensity_front`)))
  (`LightComponent.SetIntensity` (`self.SpotLight_BackRight`) (`|GetArrayItem` (`self.LightIntensity_back`)))
  (`LightComponent.SetIntensity` (`self.SpotLight_BackLeft`) (`|GetArrayItem` (`self.LightIntensity_back`))))